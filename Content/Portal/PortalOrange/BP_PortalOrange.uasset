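; BP_PortalOrange is the orange portal actor, whose surface shows whether a blue portal exists in the level.
; ActivatePortal looks up a BP_PortalBlue and sets PortalSurface to the active or inactive orange material.
; BeginPlay runs ActivatePortal and also calls it on the blue portal, if found, to refresh that side.
; The construction script repeats the same material check.
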(event `self.ReceiveBeginPlay`
  (bind _returnvalue (`GameplayStatics.GetActorOfClass` "/Game/Portal/BluePortal/BP_PortalBlue.BP_PortalBlue_C"))
  (`/Engine/EditorBlueprintResources/StandardMacros.IsValid` _returnvalue
    (:`Is Valid`
      (`self.ActivatePortal`)
      (`/Game/Portal/BluePortal/BP_PortalBlue.ActivatePortal` _returnvalue))
    (:`Is Not Valid`
      (`self.ActivatePortal`))))

(event `ActivatePortal`
  (bind _returnvalue (`GameplayStatics.GetActorOfClass` "/Game/Portal/BluePortal/BP_PortalBlue.BP_PortalBlue_C"))
  (`/Engine/EditorBlueprintResources/StandardMacros.IsValid` _returnvalue
    (:`Is Valid`
      (`PrimitiveComponent.SetMaterial` (`self.PortalSurface`) 0 "/Game/Portal/PortalOrange/M_PortalOrange.M_PortalOrange"))
    (:`Is Not Valid`
      (`PrimitiveComponent.SetMaterial` (`self.PortalSurface`) 0 "/Game/Portal/PortalOrange/M_PortalOrangeInactive.M_PortalOrangeInactive"))))

(fn `UserConstructionScript`
  (bind _returnvalue (`GameplayStatics.GetActorOfClass` "/Game/Portal/BluePortal/BP_PortalBlue.BP_PortalBlue_C"))
  (`/Engine/EditorBlueprintResources/StandardMacros.IsValid` _returnvalue
    (:`Is Valid`
      (`PrimitiveComponent.SetMaterial` (`self.PortalSurface`) 0 "/Game/Portal/PortalOrange/M_PortalOrange.M_PortalOrange"))
    (:`Is Not Valid`
      (`PrimitiveComponent.SetMaterial` (`self.PortalSurface`) 0 "/Game/Portal/PortalOrange/M_PortalOrangeInactive.M_PortalOrangeInactive"))))