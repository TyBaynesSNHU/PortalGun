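; Portal actor with a blue and orange pair of scene capture cameras that simulate the view through each portal.
; UpdateCameras moves both PSim proxies to the player camera, then copies each proxy's relative location onto the opposite colour's capture.
; Each capture faces its parent and derives a clamped FOV from the arctangent of a fixed size over distance.
; Tick is empty and the UpdateCameras call is disconnected, so nothing here runs it.
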(event `self.ReceiveTick`
  (params (DeltaSeconds :type "Float (single-precision)")))

(fn `UpdateCameras`
  (bind _bluescenecomp (`self.BlueSceneComp`))
  (bind _orangescenecomp (`self.OrangeSceneComp`))
  (`SceneComponent.K2_SetWorldLocation` (`self.PSimBlue`) (`PlayerCameraManager.GetCameraLocation` (`GameplayStatics.GetPlayerCameraManager` 0)) false false)
  (`SceneComponent.K2_SetWorldLocation` (`self.PSimOrange`) (`PlayerCameraManager.GetCameraLocation` (`GameplayStatics.GetPlayerCameraManager` 0)) false false)
  ; Update Camera Blue
  (`SceneComponent.K2_SetRelativeLocation` _bluescenecomp (`SceneComponent.RelativeLocation` (`self.PSimOrange`)) false false)
  (`SceneComponent.K2_SetWorldRotation` _bluescenecomp (`KismetMathLibrary.FindLookAtRotation` (`SceneComponent.K2_GetComponentLocation` _bluescenecomp) (`SceneComponent.K2_GetComponentLocation` (`SceneComponent.GetAttachParent` _bluescenecomp))) false false)
  (set `SceneCaptureComponent2D.FOVAngle` (`KismetMathLibrary.FClamp` (`KismetMathLibrary.DegAtan` (/ 200.0 (`KismetMathLibrary.FMax` (`KismetMathLibrary.VSize` (`SceneComponent.RelativeLocation` _bluescenecomp)) 1.0))) 5.0 180.0) _bluescenecomp)
  ; Update Camera Blue
  (`SceneComponent.K2_SetRelativeLocation` _orangescenecomp (`SceneComponent.RelativeLocation` (`self.PSimBlue`)) false false)
  (`SceneComponent.K2_SetWorldRotation` _orangescenecomp (`KismetMathLibrary.FindLookAtRotation` (`SceneComponent.K2_GetComponentLocation` _orangescenecomp) (`SceneComponent.K2_GetComponentLocation` (`SceneComponent.GetAttachParent` _orangescenecomp))) false false)
  (set `SceneCaptureComponent2D.FOVAngle` (`KismetMathLibrary.FClamp` (`KismetMathLibrary.DegAtan` (/ 200.0 (`KismetMathLibrary.FMax` (`KismetMathLibrary.VSize` (`SceneComponent.RelativeLocation` _orangescenecomp)) 1.0))) 5.0 180.0) _orangescenecomp)
  (return))

(fn `UserConstructionScript`)