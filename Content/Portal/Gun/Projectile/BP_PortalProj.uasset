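; Portal gun projectile that places a blue or orange portal where it hits.
; Construction gives the sphere a dynamic material with a blue default color.
; The hit handler reads ProjDMI's color to choose the portal type, destroys existing portals of that type, then spawns one attached to the hit component.
; ProjDMI is never assigned in these graphs, and the surface-check, attach and color-swap functions are empty stubs.
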(event `self.ReceiveBeginPlay`
  (`PrimitiveComponent.CreateDynamicMaterialInstance` (`self.Sphere`) 0 null "None"))

(event `self.ReceiveActorBeginOverlap`
  (params (OtherActor :type "Actor Object Reference")))

(event `OnActorHit_Event`
  (params (SelfActor :type "Actor Object Reference") (OtherActor :type "Actor Object Reference") (NormalImpulse :type "Vector Structure") (Hit :type "HitResult Structure (by ref)"))
  (bind (_bblockinghit _binitialoverlap _time _distance _location _impactpoint _normal _impactnormal _physmat _hitactor _hitcomponent) (`GameplayStatics.BreakHitResult` Hit))
  (bind _returnvalue (`MaterialInstanceDynamic.K2_GetVectorParameterValue` (`self.ProjDMI`) "ProjColor"))
  (if (== (`.B` (break `LinearColor` _returnvalue)) 1.0)
    (bind _outactors (`GameplayStatics.GetAllActorsOfClass` "/Game/Portal/BluePortal/BP_PortalBlue.BP_PortalBlue_C"))
    (for _array_element _outactors
      (`self.K2_DestroyActor` _array_element))
    (bind _returnvalue_2 (`|SpawnActorFromClass` "/Game/Portal/BluePortal/BP_PortalBlue.BP_PortalBlue_C" (`KismetMathLibrary.Conv_VectorToTransform` _location) "Undefined" "MultiplyWithRoot" null null))
    (`self.K2_AttachToComponent` _returnvalue_2 _hitcomponent "PortalAttach" "KeepWorld" "KeepWorld" "KeepRelative" true)
    (elif (== (`.G` (break `LinearColor` _returnvalue)) 0.2)
      (bind _outactors_2 (`GameplayStatics.GetAllActorsOfClass` "/Game/Portal/PortalOrange/BP_PortalOrange.BP_PortalOrange_C"))
      (for _array_element_2 _outactors_2
        (`self.K2_DestroyActor` _array_element_2))
      (bind _returnvalue_3 (`|SpawnActorFromClass` "/Game/Portal/PortalOrange/BP_PortalOrange.BP_PortalOrange_C" (`KismetMathLibrary.Conv_VectorToTransform` _location) "Undefined" "MultiplyWithRoot" null null))
      (`self.K2_AttachToComponent` _returnvalue_3 _hitcomponent "PortalAttach" "KeepWorld" "KeepWorld" "KeepRelative" true))))

(fn `AttachPortal`)

(fn `CheckSurface`)

(fn `SwapGunAndProjColor`)

(fn `UserConstructionScript`
  (bind _returnvalue (`PrimitiveComponent.CreateDynamicMaterialInstance` (`self.Sphere`) 0 "/Game/Portal/Gun/Projectile/M_PortalProj.M_PortalProj" "None"))
  (`MaterialInstanceDynamic.SetVectorParameterValue` _returnvalue "ProjColor" (`KismetMathLibrary.LinearColor_Blue`)))