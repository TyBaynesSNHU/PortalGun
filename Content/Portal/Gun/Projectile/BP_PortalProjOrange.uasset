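; Orange portal gun projectile that places the orange portal when it hits a near-vertical surface.
; On hit it dots the impact normal with world up; other surfaces only destroy the projectile and print a debug message.
; A valid hit replaces any existing orange portal with a new one at the impact point, attached to the hit component's PortalAttach socket with rotation snapped to it.
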(event `self.BP_OnProjectileHit`
  (params (Hit :type "HitResult Structure (by ref)"))
  (bind (_bblockinghit _binitialoverlap _time _distance _location _impactpoint _normal _impactnormal _physmat _hitactor _hitcomponent) (`GameplayStatics.BreakHitResult` Hit))
  ; Dot product to determine if surface is flat
  (if (< (`KismetMathLibrary.Abs` (`KismetMathLibrary.Dot_VectorVector` _impactnormal (0.0 0.0 1.0))) 0.1)
    (`self.K2_DestroyActor`)
    ; Spawn with a rotation transform
    (bind _returnvalue (`GameplayStatics.GetActorOfClass` "/Game/Portal/PortalOrange/BP_PortalOrange.BP_PortalOrange_C"))
    (`/Engine/EditorBlueprintResources/StandardMacros.IsValid` _returnvalue
      (:`Is Valid`
        (`self.K2_DestroyActor` _returnvalue))
      (:`Is Not Valid`
        _))
    (bind _returnvalue_2 (`|SpawnActorFromClass` "/Game/Portal/PortalOrange/BP_PortalOrange.BP_PortalOrange_C" (`KismetMathLibrary.MakeTransform` _location (`KismetMathLibrary.MakeRotFromZ` _impactnormal)) "AlwaysSpawn" "OverrideRootScale" null null))
    (`self.K2_AttachToComponent` _returnvalue_2 _hitcomponent "PortalAttach" "KeepWorld" "SnapToTarget" "KeepWorld" false)
    (else
      (`self.K2_DestroyActor`)
      (`KismetSystemLibrary.PrintString` "Dot product failed"))))

(fn `UserConstructionScript`)