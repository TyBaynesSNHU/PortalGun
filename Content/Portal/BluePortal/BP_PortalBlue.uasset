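; BP_PortalBlue is the blue half of a portal pair, showing an active or inactive surface depending on whether a BP_PortalOrange exists in the world.
; The construction script looks up the orange portal by class and sets the PortalSurface material accordingly.
; On BeginPlay it calls ActivatePortal on any orange portal found.
; Its own ActivatePortal event repeats the lookup and material swap.
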(event `self.ReceiveBeginPlay`
  (bind _returnvalue (`GameplayStatics.GetActorOfClass` "/Game/Portal/PortalOrange/BP_PortalOrange.BP_PortalOrange_C"))
  (`/Engine/EditorBlueprintResources/StandardMacros.IsValid` _returnvalue
    (:`Is Valid`
      (`/Game/Portal/PortalOrange/BP_PortalOrange.ActivatePortal` _returnvalue))))

(event `ActivatePortal`
  (bind _returnvalue (`GameplayStatics.GetActorOfClass` "/Game/Portal/PortalOrange/BP_PortalOrange.BP_PortalOrange_C"))
  (`/Engine/EditorBlueprintResources/StandardMacros.IsValid` _returnvalue
    (:`Is Valid`
      (`PrimitiveComponent.SetMaterial` (`self.PortalSurface`) 0 "/Game/Portal/BluePortal/M_BluePortal.M_BluePortal"))
    (:`Is Not Valid`
      (`PrimitiveComponent.SetMaterial` (`self.PortalSurface`) 0 "/Game/Portal/BluePortal/M_BluePortalInactive.M_BluePortalInactive"))))

(fn `UserConstructionScript`
  (bind _returnvalue (`GameplayStatics.GetActorOfClass` "/Game/Portal/PortalOrange/BP_PortalOrange.BP_PortalOrange_C"))
  (`/Engine/EditorBlueprintResources/StandardMacros.IsValid` _returnvalue
    (:`Is Valid`
      (`PrimitiveComponent.SetMaterial` (`self.PortalSurface`) 0 "/Game/Portal/BluePortal/M_BluePortal.M_BluePortal"))
    (:`Is Not Valid`
      (`PrimitiveComponent.SetMaterial` (`self.PortalSurface`) 0 "/Game/Portal/BluePortal/M_BluePortalInactive.M_BluePortalInactive"))))